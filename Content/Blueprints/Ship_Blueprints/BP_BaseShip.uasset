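; Base player spaceship that flies by physics and warps to selected targets.
; Builds stats and a runtime instance from a ship class, with debug keys cycling ship types.
; Each tick sets linear velocity from interpolated thrust plus speed-dependent pseudo-gravity, while roll and pitch apply torque.
; Warp turns toward the selection, locks it, boosts thrust by distance with camera shake and ignored WorldDynamic collision, then drops out near the target.
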(event EventBeginPlay
  (Utilities|FlowControl|Sequence
    (:then_0
      (bind _returnvalue (Game|ConstructObjectfromClass (Variables|Default|GetShip%20Class)))
      (Variables|Default|SetShip%20Stats _returnvalue))
    (:then_1
      (Variables|Default|SetThrust (/ (Variables|Default|GetMaxThrust) 0.0)))
    (:then_2
      (Default|InitializeInventory (Variables|Default|GetShip%20Stats)))
    (:then_3
      (bind _reference (Class|BPIMainPlayer|GetPlayerControllerReference(Message) (Game|GetPlayerController 0)))
      (Variables|/Game/Blueprints/MainPlayer.MainPlayer_C|SetPlayer%20Ship%20BP _reference self))
    (:then_4
      (CallFunction|SetShipStats))))

(event EventTick
  (params (DeltaSeconds :type Float%20%28single-precision%29))
  (Utilities|FlowControl|Sequence
    (:then_0
      (CallFunction|CalculateShipPhysics))
    (:then_1
      (CallFunction|SetShipPhysics))
    (:then_2
      (CallFunction|HandleShipFacing))
    (:then_3
      (if (== (Variables|Default|GetWarping) true)
        (Utilities|FlowControl|Sequence
          (:then_0
            (CallFunction|HandleWarpInitialize))
          (:then_1
            (CallFunction|HandleWarpStop))
          (:then_2
            (CallFunction|HandleWarp))
          (:then_3
            (CallFunction|HandleForwardWarpVelocity)))))))

(event Input|ActionEvents|InputActionDEBUG_Ship_Left
  (params (Key :type Key%20Structure :default "None"))
  ;[1 1 1] DEBUG - Easy way of switching between possible ship types
  (:Pressed
    (if (not (< (- (Variables|Default|GetShip%20Count) 1) 0))
      (Variables|Default|SetShip%20Count (- (Variables|Default|GetShip%20Count) 1))
      (bind _returnvalue (Game|ConstructObjectfromClass (Utilities|Array|Get(acopy) (Variables|Default|GetShips) (Variables|Default|GetShip%20Count))))
      (bind _output_get (Variables|Default|SetShip%20Stats _returnvalue))
      (CallFunction|SetShipStats)
      (Default|InitializeInventory _output_get))))

(event Input|ActionEvents|InputActionDEBUG_Ship_Right
  (params (Key :type Key%20Structure :default "None"))
  ;[1 1 1] DEBUG - Easy way of switching between possible ship types
  (:Pressed
    (if (not (> (+ (Variables|Default|GetShip%20Count) 1) (- (Utilities|Array|Length (Variables|Default|GetShips)) 1)))
      (Variables|Default|SetShip%20Count (+ (Variables|Default|GetShip%20Count) 1))
      (bind _returnvalue (Game|ConstructObjectfromClass (Utilities|Array|Get(acopy) (Variables|Default|GetShips) (Variables|Default|GetShip%20Count))))
      (bind _output_get (Variables|Default|SetShip%20Stats _returnvalue))
      (CallFunction|SetShipStats)
      (Default|InitializeInventory _output_get))))

(fn ConstructionScript)

(fn SetShipStats
  (bind _ship_stats (Variables|Default|GetShip%20Stats))
  (bind _returnvalue (Game|ConstructObjectfromClass "/Game/Blueprints/Ship_Blueprints/Ship_Stats/BP_Instanced_Ship.BP_Instanced_Ship_C"))
  (bind _returnvalue_2 (Game|ConstructObjectfromClass "/Game/Blueprints/Misc_Blueprints/BP_Inventory.BP_Inventory_C"))
  (Default|SetValues _returnvalue (Variables|/Game/Blueprints/Ship_Blueprints/Ship_Stats/BP_Ship.BP_Ship_C|GetBase%20Hull _ship_stats) (Variables|/Game/Blueprints/Ship_Blueprints/Ship_Stats/BP_Ship.BP_Ship_C|GetBase%20Armor _ship_stats) (Variables|/Game/Blueprints/Ship_Blueprints/Ship_Stats/BP_Ship.BP_Ship_C|GetBase%20Shields _ship_stats) (Variables|/Game/Blueprints/Ship_Blueprints/Ship_Stats/BP_Ship.BP_Ship_C|GetIcon _ship_stats) (Variables|/Game/Blueprints/Ship_Blueprints/Ship_Stats/BP_Ship.BP_Ship_C|GetName _ship_stats) _returnvalue_2 (Variables|/Game/Blueprints/Ship_Blueprints/Ship_Stats/BP_Ship.BP_Ship_C|GetPawn%20Class _ship_stats))
  (Variables|Default|SetCurrent%20Instance _returnvalue)
  (Variables|Default|SetMaxThrust (Variables|/Game/Blueprints/Ship_Blueprints/Ship_Stats/BP_Ship.BP_Ship_C|GetTop%20Speed _ship_stats)))

(fn MoveShip
  (params (Move%20Axis :type Float%20%28double-precision%29))
  (Utilities|FlowControl|Sequence
    (:then_0
      (if (not (Math|Float|NearlyEqual(Float) Move%20Axis 0.0 0.1))
        (Variables|Default|SetThrust (Math|Interpolation|FInterpTo (Variables|Default|GetThrust) (Math|Float|Lerp 0.0 (Variables|Default|GetMaxThrust) (/ (+ Move%20Axis 1.0) 2.0)) (Utilities|Time|GetWorldDeltaSeconds) 0.5))
        (else
          (Variables|Default|SetThrust (Math|Interpolation|FInterpTo (Variables|Default|GetThrust) 0.0 (Utilities|Time|GetWorldDeltaSeconds) 0.5)))))
    (:then_1
      (Variables|Default|SetForwardVelocity (* (Variables|Default|GetThrust) (Math|Vector|GetForwardVector (Variables|Default|GetShip)))))))

(fn RollShip
  (params (Axis%20Value :type Float%20%28double-precision%29))
  (Class|PrimitiveComponent|AddTorqueinDegrees (Variables|Default|GetShip) (* (Math|Vector|GetForwardVector (Variables|Default|GetShip)) (* Axis%20Value (Variables|Default|GetSideTorquePower))) "None" true))

(fn PitchShip
  (params (Axis%20Value :type Float%20%28double-precision%29))
  (Class|PrimitiveComponent|AddTorqueinDegrees (Variables|Default|GetShip) (* (Math|Vector|GetRightVector (Variables|Default|GetShip)) (* Axis%20Value (Variables|Default|GetForwardTorquePower))) "None" true))

(fn CalculateShipPhysics
  (bind _ship (Variables|Default|GetShip))
  (if (< (Math|Vector|VectorLength (Variables|Default|GetForwardVelocity)) (Variables|Default|GetGravityThreshold))
    (Variables|Default|SetUpwardsVelocity (* (Math|Float|Lerp 0.0 -9.8e+02 (/ (Math|Vector|VectorLength (Variables|Default|GetForwardVelocity)) (Variables|Default|GetGravityThreshold))) (Math|Vector|UnrotateVector (Math|Vector|GetUpVector _ship) (Transformation|GetWorldRotation _ship))))
    (else
      (Variables|Default|SetUpwardsVelocity (Math|Interpolation|VInterpTo (Variables|Default|GetUpwardsVelocity) "0, 0, 0" (Utilities|Time|GetWorldDeltaSeconds) 2e+01)))))

(fn SetShipPhysics
  (Physics|SetPhysicsLinearVelocity (Variables|Default|GetShip) (+ (Variables|Default|GetForwardVelocity) (Variables|Default|GetUpwardsVelocity)) false "None"))

(fn HandleShipFacing
  (if (== (Variables|Default|GetFacing) true)
    (Transformation|SetWorldRotation (Variables|Default|GetShip) (Math|Interpolation|RInterpTo (Transformation|GetWorldRotation (Variables|Default|GetShip)) (Variables|Default|GetTarget%20Rotation) (Utilities|Time|GetWorldDeltaSeconds) 0.5) false false)
    (if (Utilities|Operators|EqualEqual (Transformation|GetWorldRotation (Variables|Default|GetShip)) (Variables|Default|GetTarget%20Rotation) 2.0)
      (Transformation|SetWorldRotation (Variables|Default|GetShip) (Variables|Default|GetTarget%20Rotation) false false)
      (Variables|Default|SetFacing false)
      (Variables|Default|SetWarping true)
      (bind _reference (Class|BPIMainPlayer|GetPlayerControllerReference(Message) (Game|GetPlayerController 0)))
      (Variables|/Game/Blueprints/MainPlayer.MainPlayer_C|SetLocked%20In%20Item _reference (Variables|/Game/Blueprints/MainPlayer.MainPlayer_C|GetSelected%20Item _reference)))))

(fn HandleWarpInitialize
  (bind _reference (Class|BPIMainPlayer|GetPlayerControllerReference(Message) (Game|GetPlayerController 0)))
  (if (not (< (/ (Math|Vector|Distance(Vector) (Transformation|GetActorLocation (Variables|/Game/Blueprints/MainPlayer.MainPlayer_C|GetLocked%20In%20Item _reference)) (Transformation|GetWorldLocation (Variables|Default|GetShip))) 6.5e+02) 3e+01))
    (if (and (>= (/ (Math|Vector|Distance(Vector) (Transformation|GetActorLocation (Variables|/Game/Blueprints/MainPlayer.MainPlayer_C|GetLocked%20In%20Item _reference)) (Transformation|GetWorldLocation (Variables|Default|GetShip))) 6.5e+02) 3e+01) (< (/ (Math|Vector|Distance(Vector) (Transformation|GetActorLocation (Variables|/Game/Blueprints/MainPlayer.MainPlayer_C|GetLocked%20In%20Item _reference)) (Transformation|GetWorldLocation (Variables|Default|GetShip))) 6.5e+02) 5e+02))
      (Variables|Default|SetMaxThrust 2e+04)
      (Variables|Default|SetInWarp true)
      (CameraShakes|StartCameraShake (Game|GetPlayerCameraManager 0) "/Game/CS_Warp.CS_Warp_C" 1.0 "CameraLocal" "0, 0, 0")
      (else
        (Variables|Default|SetMaxThrust 5e+04)
        (Variables|Default|SetInWarp true)
        (CameraShakes|StartCameraShake (Game|GetPlayerCameraManager 0) "/Game/CS_Warp.CS_Warp_C" 1.0 "CameraLocal" "0, 0, 0")))))

(fn HandleWarpStop
  (bind _reference (Class|BPIMainPlayer|GetPlayerControllerReference(Message) (Game|GetPlayerController 0)))
  (if (== (Variables|Default|GetInWarp) true)
    (if (< (/ (Math|Vector|Distance(Vector) (Transformation|GetActorLocation (Variables|/Game/Blueprints/MainPlayer.MainPlayer_C|GetLocked%20In%20Item _reference)) (Transformation|GetWorldLocation (Variables|Default|GetShip))) 6.5e+02) 6.0)
      (Variables|Default|SetThrust 0.0)
      (Variables|Default|SetMaxThrust (Variables|/Game/Blueprints/Ship_Blueprints/Ship_Stats/BP_Ship.BP_Ship_C|GetTop%20Speed (Variables|Default|GetShip%20Stats)))
      (Variables|Default|SetInWarp false)
      (Variables|Default|SetWarping false)
      (Collision|SetCollisionResponsetoChannel (Variables|Default|GetShip) "ECC_WorldDynamic" "ECR_Block")
      (CameraShakes|StopCameraShake (Game|GetPlayerCameraManager 0) 0 false)
      (else
        (Collision|SetCollisionResponsetoChannel (Variables|Default|GetShip) "ECC_WorldDynamic" "ECR_Ignore")))
    (elif (== (Variables|Default|GetWarping) true)
      (if (< (/ (Math|Vector|Distance(Vector) (Transformation|GetActorLocation (Variables|/Game/Blueprints/MainPlayer.MainPlayer_C|GetLocked%20In%20Item _reference)) (Transformation|GetWorldLocation (Variables|Default|GetShip))) 6.5e+02) 2.5)
        (Variables|Default|SetWarping false)))))

(fn HandleWarp
  (if (not (Math|Float|NearlyEqual(Float) 1.0 0.0 0.1))
    (Variables|Default|SetThrust (Math|Interpolation|FInterpTo (Variables|Default|GetThrust) (Math|Float|Lerp 0.0 (Variables|Default|GetMaxThrust) (+ 1.0 1.0)) (Utilities|Time|GetWorldDeltaSeconds) 0.5))
    (else
      (Variables|Default|SetThrust (Math|Interpolation|FInterpTo (Variables|Default|GetThrust) 0.0 (Utilities|Time|GetWorldDeltaSeconds) 0.5)))))

(fn HandleForwardWarpVelocity
  (Variables|Default|SetForwardVelocity (* (Variables|Default|GetThrust) (Math|Vector|GetForwardVector (Variables|Default|GetShip)))))

(fn ActivateWarp
  (bind _reference (Class|BPIMainPlayer|GetPlayerControllerReference(Message) (Game|GetPlayerController 0)))
  (if (Utilities|Operators|NotEqual(!=) :B (Transformation|GetActorLocation (Variables|/Game/Blueprints/MainPlayer.MainPlayer_C|GetSelected%20Item _reference)))
    (Variables|Default|SetTarget%20Rotation (Math|Rotator|FindLookatRotation (Transformation|GetWorldLocation (Variables|Default|GetShip)) (Transformation|GetActorLocation (Variables|/Game/Blueprints/MainPlayer.MainPlayer_C|GetSelected%20Item _reference))))
    (Variables|Default|SetFacing true)))

(fn GetBaseShipReference
  (return self))