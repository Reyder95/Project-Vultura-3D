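; Space station instance that runs a local economy, created with contacts, item storage, a stored starter ship, one random facility and a random-quantity stockpile.
; A looping timer runs the production chain: facility output becomes market items, while consumption from the stockpile adds or removes demand listings locally and on the game instance.
; Stock additions and purchases reprice items by supply against fixed demand and median values, then broadcast market changes.
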(fn InitializeStation
  (bind _all_facilities (Variables|Default|GetAll%20Facilities))
  (CallFunction|GenerateContacts)
  (CallFunction|InitializeItemStorage)
  (bind _returnvalue (Game|ConstructObjectfromClass "/Game/Blueprints/Ship_Blueprints/Ship_Stats/BP_Instanced_Ship.BP_Instanced_Ship_C"))
  (bind _returnvalue_2 (Game|ConstructObjectfromClass "/Game/Blueprints/Misc_Blueprints/BP_Inventory.BP_Inventory_C"))
  (Default|SetValues _returnvalue 400 700 900 "/Game/Images/teapot.teapot" "Zenith Lol" _returnvalue_2 "/Game/Blueprints/Ship_Blueprints/BP_Zenith.BP_Zenith_C")
  (Utilities|Array|Add (Variables|Default|GetShip%20Storage) _returnvalue)
  (CallFunction|ConstructFacility (Utilities|Array|Get(acopy) _all_facilities (Math|Random|RandomIntegerinRange 0 (Utilities|Array|LastIndex _all_facilities))))
  (CallFunction|GenerateInitialStockpile)
  (CallFunction|RunProductionChain)
  (Utilities|Time|SetTimerbyEvent (EventDispatchers|CreateEvent :!event BPBaseStationInstanceAutoGenFunc1) 5.0 true))

(fn GenerateContacts
  (Utilities|FlowControl|Sequence
    (:then_0
      (bind _returnvalue (Game|ConstructObjectfromClass "/Game/Blueprints/Misc_Blueprints/BP_Contact.BP_Contact_C"))
      (Variables|/Game/Blueprints/Misc_Blueprints/BP_Contact.BP_Contact_C|SetName _returnvalue "Ayane Kotaka")
      (Variables|/Game/Blueprints/Misc_Blueprints/BP_Contact.BP_Contact_C|SetFaction _returnvalue "Something")
      (Variables|/Game/Blueprints/Misc_Blueprints/BP_Contact.BP_Contact_C|SetType _returnvalue "NewEnumerator0")
      (Variables|/Game/Blueprints/Misc_Blueprints/BP_Contact.BP_Contact_C|SetPortrait _returnvalue "/Game/Images/char_portrait.char_portrait")
      (Variables|Default|SetStation%20Head _returnvalue))
    (:then_1
      (for _index (range 0 (Math|Random|RandomIntegerinRange 0 4))
        (bind _returnvalue_2 (Game|ConstructObjectfromClass "/Game/Blueprints/Misc_Blueprints/BP_Contact.BP_Contact_C"))
        (Variables|/Game/Blueprints/Misc_Blueprints/BP_Contact.BP_Contact_C|SetName _returnvalue_2 "Ayane Kotaka")
        (Variables|/Game/Blueprints/Misc_Blueprints/BP_Contact.BP_Contact_C|SetFaction _returnvalue_2 "Something")
        (Variables|/Game/Blueprints/Misc_Blueprints/BP_Contact.BP_Contact_C|SetType _returnvalue_2 (Utilities|Enum|ByteToEnumStationContact (Math|Conversions|ToByte(Integer) (Math|Random|RandomIntegerinRange 1 6))))
        (Variables|/Game/Blueprints/Misc_Blueprints/BP_Contact.BP_Contact_C|SetPortrait _returnvalue_2 "/Game/Images/char_portrait.char_portrait")
        (Utilities|Array|Insert (Variables|Default|GetContacts) _returnvalue_2)))))

(fn InitializeItemStorage
  (bind _returnvalue (Game|ConstructObjectfromClass "/Game/Blueprints/Misc_Blueprints/BP_Inventory.BP_Inventory_C"))
  (Variables|Default|SetItem%20Storage _returnvalue))

(fn ConstructFacility
  (params (Facility :type BP%20Base%20Facility%20Class%20Reference))
  (bind _returnvalue (Game|ConstructObjectfromClass Facility))
  (Default|InitializeProducersandConsumers _returnvalue)
  (Utilities|Array|Add (Variables|Default|GetFacilities) _returnvalue))

(fn RunProductionChain
  (for _array_element (Variables|Default|GetFacilities)
    (bind _items (Default|Produce _array_element))
    (for _array_element_2 _items
      (CallFunction|AddItemtoMarket _array_element_2))
    (bind (_return_demand _return_remove_demand) (Default|Consume _array_element (Variables|Default|GetStockpile)))
    (bind _instance_ref (Class|BPIGameInstance|GetGameInstanceReference(Message) (Variables|Default|GetGame%20Instance)))
    (for _array_element_3 _return_demand
      (Default|AddDemand _instance_ref _array_element_3 self)
      (bind _returnvalue (Game|ConstructObjectfromClass "/Game/Blueprints/Misc_Blueprints/BP_Market_Item.BP_Market_Item_C"))
      (bind _output_get (Variables|/Game/Blueprints/Misc_Blueprints/BP_Market_Item.BP_Market_Item_C|SetItem _returnvalue _array_element_3))
      (Variables|/Game/Blueprints/Misc_Blueprints/BP_Market_Item.BP_Market_Item_C|SetQuantity _returnvalue 0)
      (Variables|/Game/Blueprints/Misc_Blueprints/BP_Market_Item.BP_Market_Item_C|SetCost _returnvalue 0)
      (Variables|/Game/Blueprints/Misc_Blueprints/BP_Market_Item.BP_Market_Item_C|SetSell _returnvalue (Math|Float|Truncate (+ (* 37.0 0.3) 37.0)))
      (Variables|/Game/Blueprints/Misc_Blueprints/BP_Market_Item.BP_Market_Item_C|SetDemand _returnvalue true)
      (bind _return (CallFunction|CheckifMarketItemExists _output_get))
      (if (not _return)
        (Utilities|Array|Add (Variables|Default|GetMarket%20Items) _returnvalue)))
    (for _array_element_4 _return_remove_demand
      (Default|RemoveDemand _instance_ref _array_element_4 self)
      (bind (_return_2 _item_index) (CallFunction|CheckifMarketItemExists _array_element_4))
      (if _return_2
        (Utilities|Array|RemoveIndex (Variables|Default|GetMarket%20Items) _item_index)))))

(fn AddItemtoMarket
  (params (Item :type BP%20Market%20Item%20Object%20Reference))
  (bind (_return _item_index) (CallFunction|CheckifMarketItemExists (Variables|/Game/Blueprints/Misc_Blueprints/BP_Market_Item.BP_Market_Item_C|GetItem Item)))
  (if _return
    (bind _output_get (Variables|/Game/Blueprints/Misc_Blueprints/BP_Market_Item.BP_Market_Item_C|SetQuantity (Utilities|Array|Get(acopy) (Variables|Default|GetMarket%20Items) _item_index) (+ (Variables|/Game/Blueprints/Misc_Blueprints/BP_Market_Item.BP_Market_Item_C|GetQuantity (Utilities|Array|Get(acopy) (Variables|Default|GetMarket%20Items) _item_index)) (Variables|/Game/Blueprints/Misc_Blueprints/BP_Market_Item.BP_Market_Item_C|GetQuantity Item))))
    (Default|AdjustPrice (Utilities|Array|Get(acopy) (Variables|Default|GetMarket%20Items) _item_index) _output_get 25 37 self (Variables|Default|GetGame%20Instance))
    (else
      (EventDispatchers|BindEventtoMarketPriceAdjusted Item (EventDispatchers|CreateEvent :!event BPBaseStationInstanceAutoGenFunc))
      (Default|AdjustPrice Item (Variables|/Game/Blueprints/Misc_Blueprints/BP_Market_Item.BP_Market_Item_C|GetQuantity Item) 25 37 self (Variables|Default|GetGame%20Instance))
      (Utilities|Array|Add (Variables|Default|GetMarket%20Items) Item)))
  (Default|CallMarketAdjusted))

(fn CheckifMarketItemExists
  (params (Item :type BP%20Base%20Item%20Object%20Reference))
  (bind (_array_element _array_index) (Utilities|Array|ForEachLoopwithBreak (Variables|Default|GetMarket%20Items) :!label _label)
    (:LoopBody
      (if (Utilities|Enum|Equal(Enum) (Variables|/Game/Blueprints/Item_Blueprints/BP_BaseItem.BP_BaseItem_C|GetItem%20Name (Variables|/Game/Blueprints/Misc_Blueprints/BP_Market_Item.BP_Market_Item_C|GetItem _array_element)) (Variables|/Game/Blueprints/Item_Blueprints/BP_BaseItem.BP_BaseItem_C|GetItem%20Name Item))
        (LocalVariables|SetExists false)
        (goto _label Break)))
    (:Completed
      (return (LocalVariables|GetExists) _array_index))))

(fn BPBaseStationInstanceAutoGenFunc
  (Default|CallMarketAdjusted))

(fn PurchaseItem
  (params (Amount :type Integer) (Item :type BP%20Base%20Item%20Object%20Reference))
  (bind (_return _item_index) (CallFunction|CheckifMarketItemExists Item))
  (if _return
    (if (<= (- (Variables|/Game/Blueprints/Misc_Blueprints/BP_Market_Item.BP_Market_Item_C|GetQuantity (Utilities|Array|Get(acopy) (Variables|Default|GetMarket%20Items) _item_index)) Amount) 0)
      (Utilities|Array|RemoveIndex (Variables|Default|GetMarket%20Items) _item_index)
      (else
        (bind _output_get (Variables|/Game/Blueprints/Misc_Blueprints/BP_Market_Item.BP_Market_Item_C|SetQuantity (Utilities|Array|Get(acopy) (Variables|Default|GetMarket%20Items) _item_index) (- (Variables|/Game/Blueprints/Misc_Blueprints/BP_Market_Item.BP_Market_Item_C|GetQuantity (Utilities|Array|Get(acopy) (Variables|Default|GetMarket%20Items) _item_index)) Amount)))
        (Default|AdjustPrice (Utilities|Array|Get(acopy) (Variables|Default|GetMarket%20Items) _item_index) _output_get 25 37 self (Variables|Default|GetGame%20Instance))))
    (Default|CallMarketAdjusted)))

(fn GenerateInitialStockpile
  (bind _returnvalue (Game|ConstructObjectfromClass "/Game/Blueprints/Misc_Blueprints/BP_Inventory.BP_Inventory_C"))
  (Variables|Default|SetStockpile _returnvalue)
  (for _array_element (Variables|Default|GetFacilities)
    (for _array_element_2 0
      (bind _returnvalue_2 (Game|ConstructObjectfromClass (Variables|/Game/Blueprints/Facility_Blueprints/BP_FacilityItem.BP_FacilityItem_C|GetItem _array_element_2)))
      (bind _returnvalue_3 (Game|ConstructObjectfromClass "/Game/Blueprints/Misc_Blueprints/BP_Inventory_Item.BP_Inventory_Item_C"))
      (Variables|/Game/Blueprints/Misc_Blueprints/BP_Inventory_Item.BP_Inventory_Item_C|SetItem _returnvalue_3 _returnvalue_2)
      (Variables|/Game/Blueprints/Misc_Blueprints/BP_Inventory_Item.BP_Inventory_Item_C|SetQuantity _returnvalue_3 (Math|Random|RandomIntegerinRange 50 100))
      (Default|AddItem (Variables|Default|GetStockpile) _returnvalue_3))))

(fn BPBaseStationInstanceAutoGenFunc1
  (CallFunction|RunProductionChain))