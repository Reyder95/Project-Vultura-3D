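; Game instance for Project Vultura that holds global space-economy state: system stations, market data and sector demand.
; On Init it creates GUID-keyed stations at randomized positions in the "Rean" system and initializes each.
; PushMarketData updates or adds price and sell entries per station and item pair.
; Demand functions add, remove, count and check requesting stations in a map keyed by item class.
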(event EventInit
  (bind _returnvalue (Game|ConstructObjectfromClass "/Game/Blueprints/Misc_Blueprints/BP_SystemStationMap.BP_SystemStationMap_C"))
  (for _index (range 0 5)
    (bind _returnvalue_2 (Game|ConstructObjectfromClass "/Game/Blueprints/Station_Blueprints/BP_BaseStationInstance.BP_BaseStationInstance_C"))
    (Variables|/Game/Blueprints/Station_Blueprints/BP_BaseStationInstance.BP_BaseStationInstance_C|SetGame%20Instance _returnvalue_2 self)
    (bind _output_get (Variables|/Game/Blueprints/Station_Blueprints/BP_BaseStationInstance.BP_BaseStationInstance_C|SetGUID _returnvalue_2 (Guid|NewGuid)))
    (bind _returnvalue_3 (Game|ConstructObjectfromClass "/Game/Blueprints/Misc_Blueprints/BP_StationWrapper.BP_StationWrapper_C"))
    (Variables|/Game/Blueprints/Misc_Blueprints/BP_StationWrapper.BP_StationWrapper_C|SetPosition%20In%20System _returnvalue_3 (Math|Vector|MakeVector (Math|Random|RandomFloatinRange -2.5e+06 2.5e+06) (Math|Random|RandomFloatinRange -1e+03 1e+03) (Math|Random|RandomFloatinRange -2.5e+06 -2.5e+06)))
    (Variables|/Game/Blueprints/Misc_Blueprints/BP_StationWrapper.BP_StationWrapper_C|SetStation _returnvalue_3 _returnvalue_2)
    (Utilities|Map|Add (Variables|/Game/Blueprints/Misc_Blueprints/BP_SystemStationMap.BP_SystemStationMap_C|GetStationMap _returnvalue) _output_get _returnvalue_3)
    (Default|InitializeStation _returnvalue_2))
  (Utilities|Map|Add (Variables|Default|GetSystem%20Station%20Map) "Rean" _returnvalue))

(fn PushMarketData
  (params (Station :type BP%20Base%20Station%20Instance%20Object%20Reference) (Item :type BP%20Base%20Item%20Object%20Reference) (Cost :type Integer) (Sell :type Integer))
  (bind (_return_value _index) (CallFunction|CheckifBothItemandStationMatch Item Station))
  (if _return_value
    (Variables|/Game/Blueprints/Misc_Blueprints/BP_GlobalMarketItem.BP_GlobalMarketItem_C|SetPrice (Utilities|Array|Get(acopy) (Variables|Default|GetMarket%20%20Data) _index) Cost)
    (Variables|/Game/Blueprints/Misc_Blueprints/BP_GlobalMarketItem.BP_GlobalMarketItem_C|SetSell (Utilities|Array|Get(acopy) (Variables|Default|GetMarket%20%20Data) _index) Sell)
    (else
      (bind _returnvalue (Game|ConstructObjectfromClass "/Game/Blueprints/Misc_Blueprints/BP_GlobalMarketItem.BP_GlobalMarketItem_C"))
      (Variables|/Game/Blueprints/Misc_Blueprints/BP_GlobalMarketItem.BP_GlobalMarketItem_C|SetStation _returnvalue Station)
      (Variables|/Game/Blueprints/Misc_Blueprints/BP_GlobalMarketItem.BP_GlobalMarketItem_C|SetItem _returnvalue Item)
      (Variables|/Game/Blueprints/Misc_Blueprints/BP_GlobalMarketItem.BP_GlobalMarketItem_C|SetPrice _returnvalue Cost)
      (Variables|/Game/Blueprints/Misc_Blueprints/BP_GlobalMarketItem.BP_GlobalMarketItem_C|SetSell _returnvalue Sell)
      (Utilities|Array|Add (Variables|Default|GetMarket%20%20Data) _returnvalue))))

(fn CheckifBothItemandStationMatch
  (params (Item :type BP%20Base%20Item%20Object%20Reference) (Station :type BP%20Base%20Station%20Instance%20Object%20Reference))
  (bind (_array_element _array_index) (Utilities|Array|ForEachLoopwithBreak (Variables|Default|GetMarket%20%20Data) :!label _label)
    (:LoopBody
      (if (== (Variables|/Game/Blueprints/Misc_Blueprints/BP_GlobalMarketItem.BP_GlobalMarketItem_C|GetStation _array_element) Station)
        (if (== (Variables|/Game/Blueprints/Misc_Blueprints/BP_GlobalMarketItem.BP_GlobalMarketItem_C|GetItem _array_element) Item)
          (LocalVariables|SetExists true)
          (goto _label Break))))
    (:Completed
      (return (LocalVariables|GetExists) _array_index))))

(fn AddDemand
  (params (Item :type BP%20Base%20Item%20Object%20Reference) (Station :type BP%20Base%20Station%20Instance%20Object%20Reference))
  (bind _returnvalue (Utilities|GetClass Item))
  (bind (_station_exists _item_exists) (CallFunction|CheckifDemandExists Item Station))
  (if _item_exists
    (if _station_exists
      (Utilities|Array|Add (Variables|/Game/Blueprints/Misc_Blueprints/BP_Station_Demand_Array.BP_Station_Demand_Array_C|GetStations (.Value (Utilities|Map|Find (Variables|Default|GetSector%20Demand%20Map) _returnvalue))) 0))
    (else
      (bind _returnvalue_2 (Game|ConstructObjectfromClass "/Game/Blueprints/Misc_Blueprints/BP_Station_Demand_Array.BP_Station_Demand_Array_C"))
      (Utilities|Array|Add (Variables|/Game/Blueprints/Misc_Blueprints/BP_Station_Demand_Array.BP_Station_Demand_Array_C|GetStations _returnvalue_2) Station)
      (Utilities|Map|Add (Variables|Default|GetSector%20Demand%20Map) _returnvalue _returnvalue_2))))

(fn CheckifDemandExists
  (params (Item :type BP%20Base%20Item%20Object%20Reference) (Station :type BP%20Base%20Station%20Instance%20Object%20Reference))
  (bind _returnvalue (Utilities|GetClass Item))
  (bind _sector_demand_map (Variables|Default|GetSector%20Demand%20Map))
  (bind (_value _returnvalue_2) (Utilities|Map|Find _sector_demand_map _returnvalue))
  (if _returnvalue_2
    (return (!= (Utilities|Array|FindItem (Variables|/Game/Blueprints/Misc_Blueprints/BP_Station_Demand_Array.BP_Station_Demand_Array_C|GetStations _value) Station) -1) true 0)
    (else
      (return false false 0))))

(fn RemoveDemand
  (params (Item :type BP%20Base%20Item%20Object%20Reference) (Station :type BP%20Base%20Station%20Instance%20Object%20Reference))
  (bind (_station_exists _item_exists _station_index) (CallFunction|CheckifDemandExists Item Station))
  (if _item_exists
    (if _station_exists
      (Utilities|Array|RemoveIndex (Variables|/Game/Blueprints/Misc_Blueprints/BP_Station_Demand_Array.BP_Station_Demand_Array_C|GetStations (.Value (Utilities|Map|Find (Variables|Default|GetSector%20Demand%20Map) (Utilities|GetClass Item)))) _station_index))))

(fn GetDemand
  (params (Item :type BP%20Base%20Item%20Object%20Reference))
  (return (Utilities|Array|Length (Variables|/Game/Blueprints/Misc_Blueprints/BP_Station_Demand_Array.BP_Station_Demand_Array_C|GetStations (.Value (Utilities|Map|Find (Variables|Default|GetSector%20Demand%20Map) (Utilities|GetClass Item)))))))

(fn CheckifAnyDemandExists
  (params (Item :type BP%20Base%20Item%20Object%20Reference))
  (return (Utilities|Map|Contains (Variables|Default|GetSector%20Demand%20Map) (Utilities|GetClass Item))))

(fn GetGameInstanceReference
  (return self))