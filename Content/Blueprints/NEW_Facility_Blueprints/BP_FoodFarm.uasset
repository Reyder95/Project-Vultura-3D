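; BP_FoodFarm is a facility Blueprint for a food farm that produces fresh food.
; It extends the parent's producer and consumer setup by constructing a facility item for a fixed amount of BP_FreshFood and adding it to the Produced list.
; A matching block that would add BP_FreshWater to the Consumed list is never executed, so this graph registers no water cost.
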(fn InitializeProducersandConsumers
  (|CallParentFunction)
  (bind _returnvalue (Game|ConstructObjectfromClass "/Game/Blueprints/Facility_Blueprints/BP_FacilityItem.BP_FacilityItem_C"))
  (Variables|/Game/Blueprints/Facility_Blueprints/BP_FacilityItem.BP_FacilityItem_C|SetItem _returnvalue "/Game/Blueprints/Item_Blueprints/TradeGoods/BP_FreshFood.BP_FreshFood_C")
  (Variables|/Game/Blueprints/Facility_Blueprints/BP_FacilityItem.BP_FacilityItem_C|SetAmount _returnvalue 5)
  (Utilities|Array|Add (Variables|Default|GetProduced) _returnvalue))