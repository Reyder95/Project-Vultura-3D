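; BP_Inventory holds an item list with stacked quantities and provides add, remove and swap operations on it.
; CheckIfItemExists searches the list by item name, and both AddItem and RemoveAmount use its result to find the matching stack.
; AddItem merges quantities or appends a new entry, RemoveAmount subtracts and deletes stacks that reach zero or below, and SwitchItems swaps two entries by index.
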(fn AddItem
  (params (Item :type BP%20Inventory%20Item%20Object%20Reference))
  (bind (_return _item_index) (CallFunction|CheckifItemExists (Variables|/Game/Blueprints/Misc_Blueprints/BP_Inventory_Item.BP_Inventory_Item_C|GetItem Item)))
  (if _return
    (Variables|/Game/Blueprints/Misc_Blueprints/BP_Inventory_Item.BP_Inventory_Item_C|SetQuantity (Utilities|Array|Get(acopy) (Variables|Default|GetItem%20List) _item_index) (+ (Variables|/Game/Blueprints/Misc_Blueprints/BP_Inventory_Item.BP_Inventory_Item_C|GetQuantity (Utilities|Array|Get(acopy) (Variables|Default|GetItem%20List) _item_index)) (Variables|/Game/Blueprints/Misc_Blueprints/BP_Inventory_Item.BP_Inventory_Item_C|GetQuantity Item)))
    (else
      (Utilities|Array|Add (Variables|Default|GetItem%20List) Item))))

(fn CheckifItemExists
  (params (Item :type BP%20Base%20Item%20Object%20Reference))
  (bind (_array_element _array_index) (Utilities|Array|ForEachLoopwithBreak (Variables|Default|GetItem%20List) :!label _label)
    (:LoopBody
      (if (Utilities|Enum|Equal(Enum) (Variables|/Game/Blueprints/Item_Blueprints/BP_BaseItem.BP_BaseItem_C|GetName Item) (Variables|/Game/Blueprints/Item_Blueprints/BP_BaseItem.BP_BaseItem_C|GetName (Variables|/Game/Blueprints/Misc_Blueprints/BP_Inventory_Item.BP_Inventory_Item_C|GetItem _array_element)))
        (LocalVariables|SetExists true)
        (goto _label Break)))
    (:Completed
      (return (LocalVariables|GetExists) _array_index))))

(fn SwitchItems
  (params (Index%201 :type Integer) (Index%202 :type Integer))
  (Utilities|Array|Swap (Variables|Default|GetItem%20List) Index%201 Index%202))

(fn RemoveAmount
  (params (Item :type BP%20Base%20Item%20Object%20Reference) (Amount :type Integer))
  (bind (_return _item_index) (CallFunction|CheckifItemExists Item))
  (if _return
    (if (<= (- (Variables|/Game/Blueprints/Misc_Blueprints/BP_Inventory_Item.BP_Inventory_Item_C|GetQuantity (Utilities|Array|Get(acopy) (Variables|Default|GetItem%20List) _item_index)) Amount) 0)
      (Utilities|Array|RemoveItem (Variables|Default|GetItem%20List) (Utilities|Array|Get(acopy) (Variables|Default|GetItem%20List) _item_index))
      (else
        (Variables|/Game/Blueprints/Misc_Blueprints/BP_Inventory_Item.BP_Inventory_Item_C|SetQuantity (Utilities|Array|Get(acopy) (Variables|Default|GetItem%20List) _item_index) (- (Variables|/Game/Blueprints/Misc_Blueprints/BP_Inventory_Item.BP_Inventory_Item_C|GetQuantity (Utilities|Array|Get(acopy) (Variables|Default|GetItem%20List) _item_index)) Amount))
        (return (- (Variables|/Game/Blueprints/Misc_Blueprints/BP_Inventory_Item.BP_Inventory_Item_C|GetQuantity (Utilities|Array|Get(acopy) (Variables|Default|GetItem%20List) _item_index)) Amount))))))