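; Base space station actor that simulates a local economy and shows an enter prompt when the player overlaps its trigger.
; BeginPlay creates placeholder contacts, storage with a starter Zenith ship, spawned facilities and a random input stockpile.
; A looping timer runs production: facility output feeds the market, while consumption adds or clears demand listings and game instance demand.
; Supply changes reprice items against fixed demand; random market generation is disconnected.
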(event OnComponentBeginOverlap(Trigger)
  (params (OverlappedComponent :type Primitive%20Component%20Object%20Reference) (OtherActor :type Actor%20Object%20Reference) (OtherComp :type Primitive%20Component%20Object%20Reference) (OtherBodyIndex :type Integer) (bFromSweep :type Boolean) (SweepResult :type Hit%20Result%20Structure%20%28by%20ref%29))
  ;[1 1 1] Handle player entering Trigger and showing "enter" text
  (CallFunction|CheckifPlayer OtherActor)
  (bind _asmain_player (Utilities|Casting|CastToMainPlayer (Game|GetPlayerController 0)))
  (Widget|SetVisibility (Variables|/Game/Blueprints/MainPlayer.MainPlayer_C|GetEnter%20Station%20Text _asmain_player) "Visible")
  (Variables|Default|SetCan%20Enter true))

(event OnComponentEndOverlap(Trigger)
  (params (OverlappedComponent :type Primitive%20Component%20Object%20Reference) (OtherActor :type Actor%20Object%20Reference) (OtherComp :type Primitive%20Component%20Object%20Reference) (OtherBodyIndex :type Integer))
  ;[1 1 1] Handle player entering Trigger and showing "enter" text
  (CallFunction|CheckifPlayer OtherActor)
  (if (Variables|Default|GetSwitched%20Ship)
    (Variables|Default|SetSwitched%20Ship false)
    (else
      (bind _asmain_player (Utilities|Casting|CastToMainPlayer (Game|GetPlayerController 0)))
      (Widget|SetVisibility (Variables|/Game/Blueprints/MainPlayer.MainPlayer_C|GetEnter%20Station%20Text _asmain_player) "Hidden")
      (Variables|Default|SetCan%20Enter false))))

(event Custom|Production%20Chain%20Event
  (CallFunction|RunProductionChain))

(event EventBeginPlay
  (CallFunction|GenerateContacts)
  (CallFunction|GenerateMarket)
  (CallFunction|InitializeItemStorage)
  (bind _returnvalue (Game|SpawnActorfromClass "/Game/Blueprints/Ship_Blueprints/BP_Zenith.BP_Zenith_C" (Math|Transform|MakeTransform "0, 0, 0" "0, 0, 0" "1.000000,1.000000,1.000000") "DontSpawnIfColliding" 0 0))
  (Utilities|Array|Add (Variables|Default|GetShip%20Storage) (Variables|/Game/Blueprints/Ship_Blueprints/BP_BaseShip.BP_BaseShip_C|GetCurrent%20Instance _returnvalue))
  (Actor|DestroyActor _returnvalue)
  (for _array_element (Variables|Default|GetGenerated%20Facilities)
    (CallFunction|ConstructFacility _array_element))
  (CallFunction|GenerateInitialStockpile)
  (CallFunction|RunProductionChain)
  (Utilities|Time|SetTimerbyEvent (delegate Custom|Production%20Chain%20Event) 5.0 true))

(fn ConstructionScript)

(fn CheckifPlayer
  (params (Pawn :type Actor%20Object%20Reference))
  (bind _aspawn (Utilities|Casting|CastToPawn Pawn))
  (Utilities|Casting|CastToPlayerController (Pawn|GetController _aspawn)))

(fn OpenUI
  (return 0))

(fn CloseUI)

(fn GenerateContacts
  (Utilities|FlowControl|Sequence
    (:then_0
      (bind _returnvalue (Game|ConstructObjectfromClass "/Game/Blueprints/Misc_Blueprints/BP_Contact.BP_Contact_C"))
      (Variables|/Game/Blueprints/Misc_Blueprints/BP_Contact.BP_Contact_C|SetName _returnvalue "Ayane Kotaka")
      (Variables|/Game/Blueprints/Misc_Blueprints/BP_Contact.BP_Contact_C|SetFaction _returnvalue "Something")
      (Variables|/Game/Blueprints/Misc_Blueprints/BP_Contact.BP_Contact_C|SetType _returnvalue "NewEnumerator0")
      (Variables|/Game/Blueprints/Misc_Blueprints/BP_Contact.BP_Contact_C|SetPortrait _returnvalue "/Game/Images/char_portrait.char_portrait")
      (Variables|Default|SetStation%20Head _returnvalue))
    (:then_1
      (for _index (range 0 (Math|Random|RandomIntegerinRange 0 4))
        (bind _returnvalue_2 (Game|ConstructObjectfromClass "/Game/Blueprints/Misc_Blueprints/BP_Contact.BP_Contact_C"))
        (Variables|/Game/Blueprints/Misc_Blueprints/BP_Contact.BP_Contact_C|SetName _returnvalue_2 "Ayane Kotaka")
        (Variables|/Game/Blueprints/Misc_Blueprints/BP_Contact.BP_Contact_C|SetFaction _returnvalue_2 "Something")
        (Variables|/Game/Blueprints/Misc_Blueprints/BP_Contact.BP_Contact_C|SetType _returnvalue_2 (Utilities|Enum|ByteToEnumStationContact (Math|Conversions|ToByte(Integer) (Math|Random|RandomIntegerinRange 1 6))))
        (Variables|/Game/Blueprints/Misc_Blueprints/BP_Contact.BP_Contact_C|SetPortrait _returnvalue_2 "/Game/Images/char_portrait.char_portrait")
        (Utilities|Array|Insert (Variables|Default|GetContacts) _returnvalue_2)))))

(fn GenerateMarket)

(fn InitializeItemStorage
  (bind _returnvalue (Game|ConstructObjectfromClass "/Game/Blueprints/Misc_Blueprints/BP_Inventory.BP_Inventory_C"))
  (Variables|Default|SetItem%20Storage _returnvalue))

(fn ConstructFacility
  (params (Facility :type BP%20Base%20Facility%20Class%20Reference))
  (bind _returnvalue (Game|SpawnActorfromClass Facility (Math|Transform|MakeTransform "0, 0, 0" "0, 0, 0" "1.000000,1.000000,1.000000") "DontSpawnIfColliding" 0 0))
  (Default|InitializeProducersandConsumers _returnvalue)
  (Utilities|Array|Add (Variables|Default|GetFacilities) _returnvalue))

(fn RunProductionChain
  (for _array_element (Variables|Default|GetFacilities)
    (bind _items (Default|Produce _array_element))
    (for _array_element_2 _items
      (CallFunction|AddItemtoMarket _array_element_2))
    (bind (_return_demand _return_remove_demand) (Default|Consume _array_element (Variables|Default|GetStockpile)))
    (bind _instance_ref (Class|BPIGameInstance|GetGameInstanceReference(Message) (Game|GetGameInstance)))
    (for _array_element_3 _return_demand
      (Default|AddDemand _instance_ref _array_element_3)
      (bind _returnvalue (Game|ConstructObjectfromClass "/Game/Blueprints/Misc_Blueprints/BP_Market_Item.BP_Market_Item_C"))
      (bind _output_get (Variables|/Game/Blueprints/Misc_Blueprints/BP_Market_Item.BP_Market_Item_C|SetItem _returnvalue _array_element_3))
      (Variables|/Game/Blueprints/Misc_Blueprints/BP_Market_Item.BP_Market_Item_C|SetQuantity _returnvalue 0)
      (Variables|/Game/Blueprints/Misc_Blueprints/BP_Market_Item.BP_Market_Item_C|SetCost _returnvalue 0)
      (Variables|/Game/Blueprints/Misc_Blueprints/BP_Market_Item.BP_Market_Item_C|SetSell _returnvalue (Math|Float|Truncate (+ (* 37.0 0.3) 37.0)))
      (Variables|/Game/Blueprints/Misc_Blueprints/BP_Market_Item.BP_Market_Item_C|SetDemand _returnvalue true)
      (bind _return (CallFunction|CheckifMarketItemExists _output_get))
      (if (not _return)
        (Utilities|Array|Add (Variables|Default|GetMarket%20Items) _returnvalue)))
    (for _array_element_4 _return_remove_demand
      (Default|RemoveDemand _instance_ref _array_element_4)
      (bind (_return_2 _item_index) (CallFunction|CheckifMarketItemExists _array_element_4))
      (if _return_2
        (Utilities|Array|RemoveIndex (Variables|Default|GetMarket%20Items) _item_index)))))

(fn AddItemtoMarket
  (params (Item :type BP%20Market%20Item%20Object%20Reference))
  (bind (_return _item_index) (CallFunction|CheckifMarketItemExists (Variables|/Game/Blueprints/Misc_Blueprints/BP_Market_Item.BP_Market_Item_C|GetItem Item)))
  (if _return
    (bind _output_get (Variables|/Game/Blueprints/Misc_Blueprints/BP_Market_Item.BP_Market_Item_C|SetQuantity (Utilities|Array|Get(acopy) (Variables|Default|GetMarket%20Items) _item_index) (+ (Variables|/Game/Blueprints/Misc_Blueprints/BP_Market_Item.BP_Market_Item_C|GetQuantity (Utilities|Array|Get(acopy) (Variables|Default|GetMarket%20Items) _item_index)) (Variables|/Game/Blueprints/Misc_Blueprints/BP_Market_Item.BP_Market_Item_C|GetQuantity Item))))
    (Default|AdjustPrice (Utilities|Array|Get(acopy) (Variables|Default|GetMarket%20Items) _item_index) _output_get 25 37 self (Game|GetGameInstance))
    (else
      (EventDispatchers|BindEventtoMarketPriceAdjusted Item (EventDispatchers|CreateEvent :!event BPBaseStationAutoGenFunc))
      (Default|AdjustPrice Item (Variables|/Game/Blueprints/Misc_Blueprints/BP_Market_Item.BP_Market_Item_C|GetQuantity Item) 25 37 self (Game|GetGameInstance))
      (Utilities|Array|Add (Variables|Default|GetMarket%20Items) Item)))
  (Default|CallMarketAdjusted))

(fn CheckifMarketItemExists
  (params (Item :type BP%20Base%20Item%20Object%20Reference))
  (bind (_array_element _array_index) (Utilities|Array|ForEachLoopwithBreak (Variables|Default|GetMarket%20Items) :!label _label)
    (:LoopBody
      (if (Utilities|Enum|Equal(Enum) (Variables|/Game/Blueprints/Item_Blueprints/BP_BaseItem.BP_BaseItem_C|GetName (Variables|/Game/Blueprints/Misc_Blueprints/BP_Market_Item.BP_Market_Item_C|GetItem _array_element)) (Variables|/Game/Blueprints/Item_Blueprints/BP_BaseItem.BP_BaseItem_C|GetName Item))
        (LocalVariables|SetExists true)
        (goto _label Break)))
    (:Completed
      (return (LocalVariables|GetExists) _array_index))))

(fn PurchaseItem
  (params (Item :type BP%20Base%20Item%20Object%20Reference) (Amount :type Integer))
  (bind (_return _item_index) (CallFunction|CheckifMarketItemExists Item))
  (if _return
    (if (<= (- (Variables|/Game/Blueprints/Misc_Blueprints/BP_Market_Item.BP_Market_Item_C|GetQuantity (Utilities|Array|Get(acopy) (Variables|Default|GetMarket%20Items) _item_index)) Amount) 0)
      (Utilities|Array|RemoveIndex (Variables|Default|GetMarket%20Items) _item_index)
      (else
        (bind _output_get (Variables|/Game/Blueprints/Misc_Blueprints/BP_Market_Item.BP_Market_Item_C|SetQuantity (Utilities|Array|Get(acopy) (Variables|Default|GetMarket%20Items) _item_index) (- (Variables|/Game/Blueprints/Misc_Blueprints/BP_Market_Item.BP_Market_Item_C|GetQuantity (Utilities|Array|Get(acopy) (Variables|Default|GetMarket%20Items) _item_index)) Amount)))
        (Default|AdjustPrice (Utilities|Array|Get(acopy) (Variables|Default|GetMarket%20Items) _item_index) _output_get 25 37 self (Game|GetGameInstance))))
    (Default|CallMarketAdjusted)))

(fn BPBaseStationAutoGenFunc
  (Default|CallMarketAdjusted))

(fn GenerateInitialStockpile
  (bind _returnvalue (Game|ConstructObjectfromClass "/Game/Blueprints/Misc_Blueprints/BP_Inventory.BP_Inventory_C"))
  (Variables|Default|SetStockpile _returnvalue)
  (for _array_element (Variables|Default|GetFacilities)
    (for _array_element_2 (Variables|/Game/Blueprints/Facility_Blueprints/BP_BaseFacility.BP_BaseFacility_C|GetConsumed _array_element)
      (bind _returnvalue_2 (Game|SpawnActorfromClass (Variables|/Game/Blueprints/Facility_Blueprints/BP_FacilityItem.BP_FacilityItem_C|GetItem _array_element_2) (Math|Transform|MakeTransform "0, 0, 0" "0, 0, 0" "1.000000,1.000000,1.000000") "Undefined" 0 0))
      (bind _returnvalue_3 (Game|ConstructObjectfromClass "/Game/Blueprints/Misc_Blueprints/BP_Inventory_Item.BP_Inventory_Item_C"))
      (Variables|/Game/Blueprints/Misc_Blueprints/BP_Inventory_Item.BP_Inventory_Item_C|SetItem _returnvalue_3 _returnvalue_2)
      (Variables|/Game/Blueprints/Misc_Blueprints/BP_Inventory_Item.BP_Inventory_Item_C|SetQuantity _returnvalue_3 (Math|Random|RandomIntegerinRange 50 100))
      (Default|AddItem (Variables|Default|GetStockpile) _returnvalue_3))))