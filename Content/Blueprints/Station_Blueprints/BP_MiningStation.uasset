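; BP_MiningStation is a station Blueprint that gives the player access to the mining station interface, extending a parent station class.
; OpenUI checks that the station is selected and enterable and the player is not already in one, then creates WBP_MiningStation linked to itself and flags the player as in a station.
; CloseUI removes the widget referenced on the MainPlayer controller, without resetting that flag here.
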(fn ConstructionScript
  (|CallParentFunction))

(fn OpenUI
  (|CallParentFunction)
  (if (Variables|Default|GetSelected)
    (bind _asmain_player (Utilities|Casting|CastToMainPlayer (Game|GetPlayerController 0)))
    (if (and (== true (Variables|Default|GetCan%20Enter)) (== (Variables|/Game/Blueprints/MainPlayer.MainPlayer_C|GetIn%20Station _asmain_player) false))
      (bind _returnvalue (UserInterface|CreateWidget "/Game/Blueprints/UserInterface/WBP_MiningStation.WBP_MiningStation_C"))
      (Variables|/Game/Blueprints/UserInterface/WBP_MiningStation.WBP_MiningStation_C|SetMining%20Station _returnvalue self)
      (UserInterface|Viewport|AddtoViewport _returnvalue 2)
      (Variables|/Game/Blueprints/MainPlayer.MainPlayer_C|SetIn%20Station _asmain_player true)
      (Variables|/Game/Blueprints/UserInterface/WBP_MiningStation.WBP_MiningStation_C|SetIs%20Open _returnvalue true)
      (return _returnvalue))))

(fn CloseUI
  (|CallParentFunction)
  (bind _asmain_player (Utilities|Casting|CastToMainPlayer (Game|GetPlayerController 0)))
  (Widget|RemovefromParent (Variables|/Game/Blueprints/MainPlayer.MainPlayer_C|GetMiningStation _asmain_player)))