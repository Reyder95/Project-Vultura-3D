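; Player controller for a spaceship game that turns input into ship flight, warp, camera control, object selection and station use.
; On BeginPlay it creates the HUD widgets and adds temporary debug items to the ship's inventory.
; Input handlers forward to the possessed BP_BaseShip, sync clicked selectables with the select table, and open a selected station's UI.
; Tick eases spring-arm zoom toward ZoomTo and polls ship speed and stats into the HUD.
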(event EventTick
  (params (DeltaSeconds :type Float%20%28single-precision%29))
  (Utilities|FlowControl|Sequence
    (:then_0
      ;[1 1 1] Handle lerping zoom (doesn't actually smooth tho)
      (bind _asbp_base_ship (Utilities|Casting|CastToBP_BaseShip (Game|Player|GetPlayerPawn 0)))
      (if true
        (Variables|/Script/Engine.SpringArmComponent|SetTargetArmLength (Variables|/Game/Blueprints/Ship_Blueprints/BP_BaseShip.BP_BaseShip_C|GetSpringArm _asbp_base_ship) (Math|Float|Lerp (Variables|/Script/Engine.SpringArmComponent|GetTargetArmLength (Variables|/Game/Blueprints/Ship_Blueprints/BP_BaseShip.BP_BaseShip_C|GetSpringArm _asbp_base_ship)) (Variables|Default|GetZoom%20To) 0.5))))
    (:then_1
      ;[1 1 1] Sets speed in UI
      (bind _asbp_base_ship_2 (Utilities|Casting|CastToBP_BaseShip (Game|Player|GetPlayerPawn 0)))
      (CallFunction|SetSpeed (Math|Float|Truncate (Variables|/Game/Blueprints/Ship_Blueprints/BP_BaseShip.BP_BaseShip_C|GetThrust _asbp_base_ship_2))))
    (:then_2
      ;[1 1 1] Sets other ship stats on UI
      (Utilities|IsValid _asbp_base_ship_2
        (:Is%20Valid
          (Default|SetStats (Variables|Default|GetHealth%20UI) (Variables|/Game/Blueprints/Ship_Blueprints/Ship_Stats/BP_Ship.BP_Ship_C|GetBase%20Hull (Variables|/Game/Blueprints/Ship_Blueprints/BP_BaseShip.BP_BaseShip_C|GetShip%20Stats _asbp_base_ship_2)) (Variables|/Game/Blueprints/Ship_Blueprints/Ship_Stats/BP_Ship.BP_Ship_C|GetBase%20Armor (Variables|/Game/Blueprints/Ship_Blueprints/BP_BaseShip.BP_BaseShip_C|GetShip%20Stats _asbp_base_ship_2)) (Variables|/Game/Blueprints/Ship_Blueprints/Ship_Stats/BP_Ship.BP_Ship_C|GetBase%20Shields (Variables|/Game/Blueprints/Ship_Blueprints/BP_BaseShip.BP_BaseShip_C|GetShip%20Stats _asbp_base_ship_2))))))))

(event EventBeginPlay
  (Utilities|FlowControl|Sequence
    (:then_0
      (CallFunction|InitializeBaseUI))
    (:then_1
      ;[1 1 1] Giving player some inventory items for debug (will be removed soon enough)
      (Utilities|FlowControl|Delay 1.0)
      (bind _returnvalue (Game|SpawnActorfromClass "/Game/Blueprints/Item_Blueprints/Ammo/BP_Bullet.BP_Bullet_C" (Math|Transform|MakeTransform "0, 0, 0" "0, 0, 0" "1.000000,1.000000,1.000000") "DontSpawnIfColliding" 0 0))
      (bind _returnvalue_2 (Game|ConstructObjectfromClass "/Game/Blueprints/Misc_Blueprints/BP_Inventory_Item.BP_Inventory_Item_C"))
      (Variables|/Game/Blueprints/Misc_Blueprints/BP_Inventory_Item.BP_Inventory_Item_C|SetItem _returnvalue_2 _returnvalue)
      (Variables|/Game/Blueprints/Misc_Blueprints/BP_Inventory_Item.BP_Inventory_Item_C|SetQuantity _returnvalue_2 37)
      (bind _asbp_base_ship (Utilities|Casting|CastToBP_BaseShip (Game|Player|GetPlayerPawn 0)))
      (Default|AddItem (Variables|/Game/Blueprints/Ship_Blueprints/Ship_Stats/BP_Instanced_Ship.BP_Instanced_Ship_C|GetInventory (Variables|/Game/Blueprints/Ship_Blueprints/BP_BaseShip.BP_BaseShip_C|GetCurrent%20Instance _asbp_base_ship)) _returnvalue_2)
      (bind _returnvalue_3 (Game|SpawnActorfromClass "/Game/Blueprints/Item_Blueprints/ActiveModules/Turrets/BP_Chaingun.BP_Chaingun_C" (Math|Transform|MakeTransform "0, 0, 0" "0, 0, 0" "1.000000,1.000000,1.000000") "DontSpawnIfColliding" 0 0))
      (bind _returnvalue_4 (Game|ConstructObjectfromClass "/Game/Blueprints/Misc_Blueprints/BP_Inventory_Item.BP_Inventory_Item_C"))
      (Variables|/Game/Blueprints/Misc_Blueprints/BP_Inventory_Item.BP_Inventory_Item_C|SetItem _returnvalue_4 _returnvalue_3)
      (Variables|/Game/Blueprints/Misc_Blueprints/BP_Inventory_Item.BP_Inventory_Item_C|SetQuantity _returnvalue_4 8)
      (Default|AddItem (Variables|/Game/Blueprints/Ship_Blueprints/Ship_Stats/BP_Instanced_Ship.BP_Instanced_Ship_C|GetInventory (Variables|/Game/Blueprints/Ship_Blueprints/BP_BaseShip.BP_BaseShip_C|GetCurrent%20Instance _asbp_base_ship)) _returnvalue_4))))

(event Input|ActionEvents|InputActionMoveCamera
  (params (Key :type Key%20Structure))
  ;[1 1 1] When move camera event fires, set Move Camera, and handle input modes to reduce lag (for some reason lol)
  (:Pressed
    (Variables|Default|SetMove%20Camera true)
    (Input|SetInputModeGameOnly self)
    (Variables|Default|SetbShowMouseCursor false)
    (bind _returnvalue (Class|WidgetLayoutLibrary|GetMousePositiononViewport))
    (Variables|Default|SetPrevious%20Mouse%20Position _returnvalue))
  (:Released
    (Variables|Default|SetMove%20Camera false)
    (Input|SetInputModeGameandUI self 0 "LockOnCapture" false)
    (Variables|Default|SetbShowMouseCursor true)
    (Class|PlayerController|SetMouseLocation (Math|Float|Truncate (.x (Variables|Default|GetPrevious%20Mouse%20Position))) (Math|Float|Truncate (.y (Variables|Default|GetPrevious%20Mouse%20Position))))))

(event Input|ActionEvents|InputActionZoomIn
  (params (Key :type Key%20Structure))
  ;[1 1 1] Handle Zoom In
  (:Pressed
    (bind _asbp_base_ship (Utilities|Casting|CastToBP_BaseShip (Game|Player|GetPlayerPawn 0)))
    (if (or (<= 1e+02 (Variables|Default|GetZoom%20To)) (<= 1e+02 (Variables|/Script/Engine.SpringArmComponent|GetTargetArmLength (Variables|/Game/Blueprints/Ship_Blueprints/BP_BaseShip.BP_BaseShip_C|GetSpringArm _asbp_base_ship))))
      (if (<= 1e+02 (- (Variables|/Script/Engine.SpringArmComponent|GetTargetArmLength (Variables|/Game/Blueprints/Ship_Blueprints/BP_BaseShip.BP_BaseShip_C|GetSpringArm _asbp_base_ship)) (Variables|Default|GetZoom%20Sensitivity)))
        (Variables|Default|SetZoom%20To (- (Variables|/Script/Engine.SpringArmComponent|GetTargetArmLength (Variables|/Game/Blueprints/Ship_Blueprints/BP_BaseShip.BP_BaseShip_C|GetSpringArm _asbp_base_ship)) (Variables|Default|GetZoom%20Sensitivity)))
        (else
          (Variables|Default|SetZoom%20To 2e+02))))))

(event Input|ActionEvents|InputActionZoomOut
  (params (Key :type Key%20Structure))
  ;[1 1 1] Zoom Camera Out
  (:Pressed
    (bind _asbp_base_ship (Utilities|Casting|CastToBP_BaseShip (Game|Player|GetPlayerPawn 0)))
    (if (or (<= (Variables|Default|GetZoom%20To) 5e+03) (<= (Variables|/Script/Engine.SpringArmComponent|GetTargetArmLength (Variables|/Game/Blueprints/Ship_Blueprints/BP_BaseShip.BP_BaseShip_C|GetSpringArm _asbp_base_ship)) 5e+03))
      (if (<= 0.0 (+ (Variables|/Script/Engine.SpringArmComponent|GetTargetArmLength (Variables|/Game/Blueprints/Ship_Blueprints/BP_BaseShip.BP_BaseShip_C|GetSpringArm _asbp_base_ship)) (Variables|Default|GetZoom%20Sensitivity)))
        (Variables|Default|SetZoom%20To (+ (Variables|/Script/Engine.SpringArmComponent|GetTargetArmLength (Variables|/Game/Blueprints/Ship_Blueprints/BP_BaseShip.BP_BaseShip_C|GetSpringArm _asbp_base_ship)) (Variables|Default|GetZoom%20Sensitivity)))
        (else
          (Variables|Default|SetZoom%20To 5e+03))))))

(event Input|ActionEvents|InputActionUse
  (params (Key :type Key%20Structure))
  (bind _selected_item (Variables|Default|GetSelected%20Item))
  ;[1 1 1] Enter station by pressing the "Use" key
  (:Pressed
    (Utilities|IsValid _selected_item
      (:Is%20Valid
        (bind _asbp_base_station (Utilities|Casting|CastToBP_BaseStation _selected_item))
        (bind _ui_reference (Default|OpenUI _asbp_base_station))
        (Variables|Default|SetMiningStation _ui_reference)))))

(event Input|ActionEvents|InputActionInventory
  (params (Key :type Key%20Structure))
  (bind _inventory_ui (Variables|Default|GetInventory%20UI))
  ;[1 1 1] Inventory button pressed
  (:Pressed
    (if (== (Math|Conversions|ToInteger(Byte) (Widget|GetVisibility _inventory_ui)) 0)
      (Widget|SetVisibility _inventory_ui "Hidden")
      (Default|RemoveInventory _inventory_ui)
      (else
        (Default|FillInventory _inventory_ui)
        (Widget|SetVisibility _inventory_ui "Visible")))))

(event Input|ActionEvents|InputActionSelectObject
  (params (Key :type Key%20Structure))
  ;[1 1 1] Select an object by clicking on the object in 3D space
  (:Pressed
    (bind _asbp_base_selectable (Utilities|Casting|CastToBP_BaseSelectable (.HitActor (Collision|BreakHitResult (.HitResult (Game|Player|GetHitResultUnderCursorbyChannel "TraceTypeQuery1" true))))))
    (Utilities|IsValid (Variables|Default|GetSelected%20Item)
      (:Is%20Valid
        (if (== _asbp_base_selectable (Variables|Default|GetSelected%20Item))
          (for _array_element (Class|PanelWidget|GetAllChildren (Variables|/Game/Blueprints/UserInterface/WBP_Select_Table.WBP_Select_Table_C|GetMainScrollbox (Variables|Default|GetSelect%20Table)))
            (bind _aswbp_select_entry (Utilities|Casting|CastToWBP_Select_Entry _array_element))
            (if (== (Variables|Default|GetSelected%20Item) (Variables|/Game/Blueprints/UserInterface/WBP_Select_Entry.WBP_Select_Entry_C|GetObject _aswbp_select_entry))
              (Default|SelectObject _aswbp_select_entry)))
          (else
            (bind _output_get (Variables|Default|SetSelected%20Item _asbp_base_selectable :!label _label))
            (for _array_element_2 (Class|PanelWidget|GetAllChildren (Variables|/Game/Blueprints/UserInterface/WBP_Select_Table.WBP_Select_Table_C|GetMainScrollbox (Variables|Default|GetSelect%20Table)))
              (bind _aswbp_select_entry_2 (Utilities|Casting|CastToWBP_Select_Entry _array_element_2))
              (if (== (Variables|/Game/Blueprints/UserInterface/WBP_Select_Entry.WBP_Select_Entry_C|GetObject _aswbp_select_entry_2) _output_get)
                (Default|SelectObject _aswbp_select_entry_2))))))
      (:Is%20Not%20Valid
        (goto _label)))))

(event Input|ActionEvents|InputActionActivateWarp
  (params (Key :type Key%20Structure))
  ;[1 1 1] Activate warp drive
  (:Pressed
    (bind _asbp_base_ship (Utilities|Casting|CastToBP_BaseShip (Game|Player|GetPlayerPawn 0)))
    (Default|ActivateWarp _asbp_base_ship)))

(event Input|AxisEvents|InputAxisMoveY
  (params (AxisValue :type Float%20%28single-precision%29))
  ;[1 1 1] Move ship forward
  (bind _asbp_base_ship (Utilities|Casting|CastToBP_BaseShip (Game|Player|GetPlayerPawn 0)))
  (Default|MoveShip _asbp_base_ship AxisValue))

(event Input|AxisEvents|InputAxisPitch
  (params (AxisValue :type Float%20%28single-precision%29))
  ;[1 1 1] Pitch the ship
  (bind _asbp_base_ship (Utilities|Casting|CastToBP_BaseShip (Game|Player|GetPlayerPawn 0)))
  (Default|PitchShip _asbp_base_ship AxisValue))

(event Input|AxisEvents|InputAxisRoll
  (params (AxisValue :type Float%20%28single-precision%29))
  ;[1 1 1] Roll ship
  (bind _asbp_base_ship (Utilities|Casting|CastToBP_BaseShip (Game|Player|GetPlayerPawn 0)))
  (Default|RollShip _asbp_base_ship AxisValue))

(event Input|MouseEvents|MouseX
  (params (AxisValue :type Float%20%28single-precision%29))
  ;[1 1 1] Rotate Camera based on mouse position. Only works when able to move camera
  (bind _asbp_base_ship (Utilities|Casting|CastToBP_BaseShip (Game|Player|GetPlayerPawn 0)))
  (if (== (Variables|Default|GetMove%20Camera) true)
    (Pawn|Input|AddControllerYawInput _asbp_base_ship AxisValue)))

(event Input|MouseEvents|MouseY
  (params (AxisValue :type Float%20%28single-precision%29))
  (bind _returnvalue (Game|Player|GetPlayerPawn 0))
  (bind _returnvalue_2 (Pawn|GetControlRotation :!class /Script/Engine.Controller))
  ;[1 1 1] Input Event to move ship forward
  (bind _asbp_base_ship (Utilities|Casting|CastToBP_BaseShip _returnvalue))
  (if (== (Variables|Default|GetMove%20Camera) true)
    (Pawn|Input|AddControllerPitchInput _returnvalue (/ AxisValue -1.0))
    (Transformation|SetRelativeRotation (Variables|/Game/Blueprints/Ship_Blueprints/BP_BaseShip.BP_BaseShip_C|GetSpringArm _asbp_base_ship) (Math|Rotator|MakeRotator 0.0 (.pitch _returnvalue_2) (.yaw _returnvalue_2)) false false)))

(fn ConstructionScript)

(fn SetSpeed
  (params (Speed :type Integer))
  (Rendering|Components|TextRender|SetText (Variables|/Game/Blueprints/UserInterface/WBP_Speed_UI.WBP_Speed_UI_C|GetSpeed (Variables|Default|GetSpeed%20UI)) (Utilities|Text|ToText(Integer) Speed)))

(fn InitializeBaseUI
  (Utilities|FlowControl|Sequence
    (:then_0
      (bind _returnvalue (UserInterface|CreateWidget "/Game/Blueprints/UserInterface/WBP_Speed_UI.WBP_Speed_UI_C"))
      (bind _output_get (Variables|Default|SetSpeed%20UI _returnvalue))
      (UserInterface|Viewport|AddtoViewport _output_get 0))
    (:then_1
      (bind _returnvalue_2 (UserInterface|CreateWidget "/Game/Blueprints/UserInterface/WBP_Select_Table.WBP_Select_Table_C"))
      (bind _output_get_2 (Variables|Default|SetSelect%20Table _returnvalue_2))
      (UserInterface|Viewport|AddtoViewport _output_get_2 1))
    (:then_2
      (bind _returnvalue_3 (UserInterface|CreateWidget "/Game/Blueprints/UserInterface/WBP_Ship_Health.WBP_Ship_Health_C"))
      (bind _output_get_3 (Variables|Default|SetHealth%20UI _returnvalue_3))
      (UserInterface|Viewport|AddtoViewport _output_get_3 0))
    (:then_3
      (bind _returnvalue_4 (UserInterface|CreateWidget "/Game/Blueprints/UserInterface/WBP_Player_Inventory.WBP_Player_Inventory_C"))
      (bind _output_get_4 (Variables|Default|SetInventory%20UI _returnvalue_4))
      (UserInterface|Viewport|AddtoViewport _output_get_4 0)
      (Widget|SetVisibility _output_get_4 "Hidden"))
    (:then_4
      (bind _returnvalue_5 (UserInterface|CreateWidget "/Game/Blueprints/UserInterface/WBP_Station_Enter.WBP_Station_Enter_C"))
      (bind _output_get_5 (Variables|Default|SetEnter%20Station%20Text _returnvalue_5))
      (UserInterface|Viewport|AddtoViewport _output_get_5 0)
      (Widget|SetVisibility _output_get_5 "Hidden"))))