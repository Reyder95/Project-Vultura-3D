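; BP_BaseFacility is a base facility that produces market items and consumes items from a stockpile.
; Produce turns each Produced entry into a BP_Market_Item with item and quantity, then adds it to CurrentProduction.
; Consume removes each Consumed amount from the stockpile and toggles Demand when the returned amount crosses a threshold relative to consumption, returning added and removed demands.
; InitializeProducersAndConsumers is an empty stub.
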(fn InitializeProducersandConsumers)

(fn Produce
  (for _array_element (Variables|Default|GetProduced)
    (bind _returnvalue (Game|ConstructObjectfromClass (Variables|/Game/Blueprints/Facility_Blueprints/BP_FacilityItem.BP_FacilityItem_C|GetItem _array_element)))
    (bind _returnvalue_2 (Game|ConstructObjectfromClass "/Game/Blueprints/Misc_Blueprints/BP_Market_Item.BP_Market_Item_C"))
    (Variables|/Game/Blueprints/Misc_Blueprints/BP_Market_Item.BP_Market_Item_C|SetItem _returnvalue_2 _returnvalue)
    (Variables|/Game/Blueprints/Misc_Blueprints/BP_Market_Item.BP_Market_Item_C|SetQuantity _returnvalue_2 (Variables|/Game/Blueprints/Facility_Blueprints/BP_FacilityItem.BP_FacilityItem_C|GetAmount _array_element))
    (Utilities|Array|Add (LocalVariables|GetCurrent%20Production) _returnvalue_2))
  (return (LocalVariables|GetCurrent%20Production)))

(fn Consume
  (params (Stockpile :type BP%20Inventory%20Object%20Reference))
  (for _array_element (Variables|Default|GetConsumed)
    (bind _returnvalue (Game|ConstructObjectfromClass (Variables|/Game/Blueprints/Facility_Blueprints/BP_FacilityItem.BP_FacilityItem_C|GetItem _array_element)))
    (bind _remaining (Default|RemoveAmount Stockpile _returnvalue (Variables|/Game/Blueprints/Facility_Blueprints/BP_FacilityItem.BP_FacilityItem_C|GetAmount _array_element)))
    (if (or (<= _remaining 0) (<= (/ _remaining (Math|Conversions|ToFloat(Integer) (Variables|/Game/Blueprints/Facility_Blueprints/BP_FacilityItem.BP_FacilityItem_C|GetAmount _array_element))) 3.0))
      (if (not (Variables|/Game/Blueprints/Facility_Blueprints/BP_FacilityItem.BP_FacilityItem_C|GetDemand _array_element))
        (Variables|/Game/Blueprints/Facility_Blueprints/BP_FacilityItem.BP_FacilityItem_C|SetDemand _array_element true)
        (Utilities|Array|Add (LocalVariables|GetDemand%20Array) _returnvalue))
      (elif (Variables|/Game/Blueprints/Facility_Blueprints/BP_FacilityItem.BP_FacilityItem_C|GetDemand _array_element)
        (Variables|/Game/Blueprints/Facility_Blueprints/BP_FacilityItem.BP_FacilityItem_C|SetDemand _array_element false)
        (Utilities|Array|Add (LocalVariables|GetRemove%20Demand%20Array) _returnvalue))))
  (return (LocalVariables|GetDemand%20Array) (LocalVariables|GetRemove%20Demand%20Array)))