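; BP_AmmoFactory is a facility Blueprint that defines an ammo factory producing bullets and consuming fresh food.
; It overrides InitializeProducersAndConsumers, calls the parent version, then constructs facility item objects pairing an item with an amount.
; The bullet entry is added to the Produced collection and the fresh food entry to Consumed, with no production logic of its own.
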(fn InitializeProducersandConsumers
  (|CallParentFunction)
  (bind _returnvalue (Game|ConstructObjectfromClass "/Game/Blueprints/Facility_Blueprints/BP_FacilityItem.BP_FacilityItem_C"))
  (Variables|/Game/Blueprints/Facility_Blueprints/BP_FacilityItem.BP_FacilityItem_C|SetItem _returnvalue "/Game/Blueprints/Item_Blueprints/Ammo/BP_Bullet.BP_Bullet_C")
  (Variables|/Game/Blueprints/Facility_Blueprints/BP_FacilityItem.BP_FacilityItem_C|SetAmount _returnvalue 5)
  (Utilities|Array|Add (Variables|Default|GetProduced) _returnvalue)
  (bind _returnvalue_2 (Game|ConstructObjectfromClass "/Game/Blueprints/Facility_Blueprints/BP_FacilityItem.BP_FacilityItem_C"))
  (Variables|/Game/Blueprints/Facility_Blueprints/BP_FacilityItem.BP_FacilityItem_C|SetItem _returnvalue_2 "/Game/Blueprints/Item_Blueprints/TradeGoods/BP_FreshFood.BP_FreshFood_C")
  (Variables|/Game/Blueprints/Facility_Blueprints/BP_FacilityItem.BP_FacilityItem_C|SetAmount _returnvalue_2 10)
  (Utilities|Array|Add (Variables|Default|GetConsumed) _returnvalue_2))