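; Base ammo item Blueprint that gives each generated ammo item a random ammo type.
; Its Generate Item override runs the parent generation, then constructs an object from a uniformly random class in PossibleTypes and stores it as AmmoType.
; It returns the parent's result unchanged, and its construction script only calls the parent.
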(fn ConstructionScript
  (|CallParentFunction))

(fn GenerateItem
  (bind _possibletypes (Variables|Default|GetPossibleTypes))
  (bind _item (|CallParentFunction))
  (bind _returnvalue (Game|ConstructObjectfromClass (Utilities|Array|Get(acopy) _possibletypes (Math|Random|RandomIntegerinRange 0 (- (Utilities|Array|Length _possibletypes) 1)))))
  (Variables|Default|SetAmmo%20Type _returnvalue)
  (return _item))