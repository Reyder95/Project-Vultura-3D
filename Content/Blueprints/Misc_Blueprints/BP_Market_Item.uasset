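; BP_Market_Item recalculates an item's buy and sell prices at a station from supply and sector demand.
; AdjustPrice reads demand as the item class's station count in the GameInstance's SectorDemandMap, ignoring its Demand input.
; Integer diminishing-returns formulas turn supply and demand into a ratio that scales MedianPrice, with sell price 30% below cost.
; It pushes both prices to the GameInstance and calls MarketPriceAdjusted.
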(fn AdjustPrice
  (params (Supply :type Integer) (Demand :type Integer) (Median%20Price :type Integer) (Station :type BP%20Base%20Station%20Instance%20Object%20Reference) (Game%20Instance :type Game%20Instance%20Object%20Reference))
  (bind _instance_ref (Class|BPIGameInstance|GetGameInstanceReference(Message) Game%20Instance))
  (bind (_station_exists _item_exists) (Default|CheckifDemandExists _instance_ref (Variables|Default|GetItem) Station))
  (if (and _item_exists _station_exists)
    (LocalVariables|SetSector%20Demand (Utilities|Array|Length (Variables|/Game/Blueprints/Misc_Blueprints/BP_Station_Demand_Array.BP_Station_Demand_Array_C|GetStations (.Value (Utilities|Map|Find (Variables|/Game/Blueprints/ProjectVultura_GameInstance.ProjectVultura_GameInstance_C|GetSector%20Demand%20Map _instance_ref) (Utilities|GetClass (Variables|Default|GetItem)))))))
    (else
      (LocalVariables|SetSector%20Demand 0)))
  (bind _relative_demand (CallFunction|CalculateRelativeDemand (LocalVariables|GetSector%20Demand)))
  (bind _relative_supply (CallFunction|CalculateRelativeSupply Supply))
  (bind _output_get (Variables|Default|SetCost (Math|Float|Truncate (* (/ (Math|Conversions|ToFloat(Integer) _relative_supply) (Math|Conversions|ToFloat(Integer) _relative_demand)) Median%20Price))))
  (bind _output_get_2 (Variables|Default|SetSell (Math|Float|Floor (- (Math|Conversions|ToFloat(Integer) _output_get) (* (Math|Conversions|ToFloat(Integer) _output_get) 0.3)))))
  (Default|PushMarketData _instance_ref Station (Variables|Default|GetItem) _output_get _output_get_2)
  (Default|CallMarketPriceAdjusted))

(fn CalculateRelativeSupply
  (params (Supply :type Integer))
  (bind _returnvalue (+ Supply 5))
  (return (/ (+ _returnvalue 100) _returnvalue)))

(fn CalculateRelativeDemand
  (params (Demand :type Integer))
  (bind _returnvalue (* Demand 3))
  (bind _returnvalue_2 (+ _returnvalue 10))
  (return (/ (+ _returnvalue_2 100) _returnvalue_2)))

(fn GetGameInstanceReference
  (return 0))