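; BP_FoodFarm is a facility Blueprint that produces fresh food from fresh water.
; It extends the parent's producer and consumer setup, adding constructed BP_FacilityItem entries to the Produced and Consumed lists, each holding an item and an amount.
; Its event graph and construction script add no logic of their own.
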(event EventBeginPlay
  (|CallParentFunction) ; This node is disabled and will not be called.\nDrag off pins to build functionality.
)

(event Collision|EventActorBeginOverlap
  (params (OtherActor :type Actor%20Object%20Reference))
  (|CallParentFunction OtherActor) ; This node is disabled and will not be called.\nDrag off pins to build functionality.
)

(event EventTick
  (params (DeltaSeconds :type Float%20%28single-precision%29))
  (|CallParentFunction DeltaSeconds) ; This node is disabled and will not be called.\nDrag off pins to build functionality.
)

(fn ConstructionScript
  (|CallParentFunction))

(fn InitializeProducersandConsumers
  (|CallParentFunction)
  (bind _returnvalue (Game|ConstructObjectfromClass "/Game/Blueprints/Facility_Blueprints/BP_FacilityItem.BP_FacilityItem_C"))
  (Variables|/Game/Blueprints/Facility_Blueprints/BP_FacilityItem.BP_FacilityItem_C|SetItem _returnvalue "/Game/Blueprints/Item_Blueprints/Trade_Goods/BP_Fresh_Food.BP_Fresh_Food_C")
  (Variables|/Game/Blueprints/Facility_Blueprints/BP_FacilityItem.BP_FacilityItem_C|SetAmount _returnvalue 5)
  (Utilities|Array|Add (Variables|Default|GetProduced) _returnvalue)
  (bind _returnvalue_2 (Game|ConstructObjectfromClass "/Game/Blueprints/Facility_Blueprints/BP_FacilityItem.BP_FacilityItem_C"))
  (Variables|/Game/Blueprints/Facility_Blueprints/BP_FacilityItem.BP_FacilityItem_C|SetItem _returnvalue_2 "/Game/Blueprints/Item_Blueprints/Trade_Goods/BP_Fresh_Water.BP_Fresh_Water_C")
  (Variables|/Game/Blueprints/Facility_Blueprints/BP_FacilityItem.BP_FacilityItem_C|SetAmount _returnvalue_2 13)
  (Utilities|Array|Add (Variables|Default|GetConsumed) _returnvalue_2))